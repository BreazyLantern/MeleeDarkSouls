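; Actor component that handles sword hit detection, dealing damage to pawns the blade touches.
; While the weapon is active, Tick runs a multi sphere trace between the sword mesh's Start and End sockets, sized by the sword, with debug drawing on.
; Each new hit actor takes the sword's damage and joins an ignore list to prevent repeat hits; this graph never clears that list.
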(event EventBeginPlay)

(event EventTick
  (params (DeltaSeconds :type Float%20%28single-precision%29))
  (bind _swordref (Variables|Default|GetSwordRef))
  (bind _skeletalmesh (Variables|/Game/CourseWork/Equipment/BP_BaseSword.BP_BaseSword_C|GetSkeletalMesh _swordref))
  (if (Variables|Default|GetWeaponActive)
    (bind _outhits (Collision|MultiSphereTraceForObjects (Transformation|GetSocketLocation _skeletalmesh "Start") (Transformation|GetSocketLocation _skeletalmesh "End") (Variables|/Game/CourseWork/Equipment/BP_BaseSword.BP_BaseSword_C|Gettracesize _swordref) (Utilities|Array|MakeArray "ObjectTypeQuery3") false (Variables|Default|GetEnemy) "ForDuration"))
    (for _array_element _outhits
      (if (not (Utilities|Array|ContainsItem (Variables|Default|GetActorsToIgnore) (.HitActor (Collision|BreakHitResult _array_element))))
        (Game|Damage|ApplyDamage (.HitActor (Collision|BreakHitResult _array_element)) (Variables|/Game/CourseWork/Equipment/BP_BaseSword.BP_BaseSword_C|GetswordDamage (Variables|Default|GetSwordRef)) 0 (Components|GetOwner))
        (Utilities|Array|Add (Variables|Default|GetActorsToIgnore) (.HitActor (Collision|BreakHitResult _array_element)))))))