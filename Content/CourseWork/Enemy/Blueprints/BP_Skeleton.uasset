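; Skeleton enemy character that fights the player with a socket-attached sword and supports lock-on targeting.
; Runs a behavior tree, pushing a behavior enum to its blackboard on sight, damage and the player leaving its sphere.
; Trace and rotating components receive sword and target references, while attacks play random montages.
; Damage triggers a hit reaction and health bar, or death that stops AI and releases the player's lock-on if targeted.
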(event OnSeePawn(PawnSensing)
  (params (Pawn :type Pawn%20Object%20Reference))
  ;[1 1 1] Sight
  (if (and (== Pawn (Variables|Ref|GetAs%20BP%20Third%20Person%20Character)) (Utilities|Enum|NotEqual(Enum) (Variables|State|GetBehavior) "NewEnumerator0"))
    (Variables|State|SetBehavior "NewEnumerator3")
    (AI|Components|Blackboard|SetValueasEnum (AI|GetBlackboard 0) (Utilities|Name|MakeLiteralName "EBehavior") (Variables|State|GetBehavior))))

(event OnComponentEndOverlap(Sphere)
  (params (OverlappedComponent :type Primitive%20Component%20Object%20Reference) (OtherActor :type Actor%20Object%20Reference) (OtherComp :type Primitive%20Component%20Object%20Reference) (OtherBodyIndex :type Integer))
  ;[1 1 1] Escape Enemy
  (Utilities|Casting|CastToBP_ThirdPersonCharacter OtherActor)
  (Variables|State|SetBehavior "NewEnumerator1")
  (AI|Components|Blackboard|SetValueasEnum (AI|GetBlackboard 0) (Utilities|Name|MakeLiteralName "EBehavior") (Variables|State|GetBehavior))
  (Rendering|SetVisibility (Variables|Default|GetWBHealthBar) false false))

(event Custom|Attack
  ;[1 1 1] Attack
  (bind _returnvalue (Animation|PlayAnimMontage (.OutItem (Utilities|Array|Random (Variables|Ref|GetAttackAnimations))) 1.0 "None"))
  (Variables|Combat|SetAttackLength _returnvalue))

(event Custom|ClearHitActors
  ;[1 1 1] Clear
  (Utilities|Array|Clear (Variables|/Game/CourseWork/Equipment/BPC_TraceComponent.BPC_TraceComponent_C|GetActorsToIgnore (Variables|Default|GetBPC_TraceComponent))))

(event EventBeginPlay
  (Utilities|FlowControl|Sequence
    (:then_0
      ;[1 1 1] Behavior tree
      (AI|RunBehaviorTree (AI|GetAIController self) "/Game/CourseWork/Enemy/BehaviorTree/BT_Skeleton.BT_Skeleton"))
    (:then_1
      ;[1 1 1] Spawn Sword
      (bind _returnvalue (Game|SpawnActorfromClass (Variables|Combat|Getsword) (Transformation|GetSocketTransform (Variables|Character|GetMesh) "sword" "RTS_World") "Undefined" "MultiplyWithRoot" 0 0))
      (bind _output_get (Variables|Combat|SetAs%20BP%20Base%20Sword _returnvalue))
      (Transformation|AttachComponentToComponent _output_get (Variables|Character|GetMesh) "sword" "SnapToTarget" "SnapToTarget" "SnapToTarget" true)
      (Variables|/Game/CourseWork/Equipment/BPC_TraceComponent.BPC_TraceComponent_C|SetSwordRef (Variables|Default|GetBPC_TraceComponent) _output_get))
    (:then_2
      ;[1 1 1] Ref values
      (bind _asbp_third_person_character (Utilities|Casting|CastToBP_ThirdPersonCharacter (Game|GetPlayerCharacter 0)))
      (Variables|Ref|SetAs%20BP%20Third%20Person%20Character _asbp_third_person_character)
      (AI|Components|Blackboard|SetValueasEnum (AI|GetBlackboard 0) (Utilities|Name|MakeLiteralName "EBehavior") (Variables|State|GetBehavior)))
    (:then_3
      (Variables|/Game/CourseWork/Equipment/BPC_RotatingComponent.BPC_RotatingComponent_C|SetTarget (Variables|Default|GetBPC_RotatingComponent) (Game|GetPlayerCharacter 0)))
    (:then_4
      (bind _outactors (Actor|GetAllActorswithTag "Enemy"))
      (Variables|/Game/CourseWork/Equipment/BPC_TraceComponent.BPC_TraceComponent_C|SetEnemy (Variables|Default|GetBPC_TraceComponent) _outactors))
    (:then_5
      (Variables|Init|SetMaxHealth (Variables|Init|GetHealth)))
    (:then_6
      (bind _aswb_skeleton_health_bar (Utilities|Casting|CastToWB_SkeletonHealthBar (UserInterface|GetWidget (Variables|Default|GetWBHealthBar))))
      (bind _output_get_2 (Variables|Ref|SetHealthBarRef _aswb_skeleton_health_bar))
      (Variables|/Game/CourseWork/Enemy/Blueprints/WB_SkeletonHealthBar.WB_SkeletonHealthBar_C|SetSkeleRef _output_get_2 self))))

(event Collision|EventActorBeginOverlap
  (params (OtherActor :type Actor%20Object%20Reference)))

(event EventTick
  (params (DeltaSeconds :type Float%20%28single-precision%29)))

(event Game|Damage|EventAnyDamage
  (params (Damage :type Float%20%28single-precision%29) (DamageType :type Damage%20Type%20Object%20Reference) (InstigatedBy :type Controller%20Object%20Reference) (DamageCauser :type Actor%20Object%20Reference))
  (bind _as_bp_third_person_character (Variables|Ref|GetAs%20BP%20Third%20Person%20Character))
  (bind _targetactor (Variables|/Game/CourseWork/ThirdPerson/Blueprints/BP_ThirdPersonCharacter.BP_ThirdPersonCharacter_C|GetTargetActor _as_bp_third_person_character))
  ;[1 1 1] Take Damage
  (Variables|State|SetBehavior "NewEnumerator0")
  (AI|Components|Blackboard|SetValueasEnum (AI|GetBlackboard 0) (Utilities|Name|MakeLiteralName "EBehavior") (Variables|State|GetBehavior))
  (bind _output_get (Variables|Init|SetHealth (- (Variables|Init|GetHealth) Damage)))
  (if (<= _output_get 0.0)
    (Utilities|FlowControl|DoOnce false
      (:Completed
        (AI|Logic|StopLogic (Variables|/Script/AIModule.AIController|GetBrainComponent (AI|GetAIController self)) "")
        (Variables|Death|SetEnemyDead? true)
        (Animation|PlayAnimMontage "/Game/CourseWork/Enemy/Animations/SkeleDeath_Montage.SkeleDeath_Montage" 1.0 "None")
        (Utilities|IsValid _targetactor
          (:Is%20Valid
            (if (== _targetactor self)
              (Default|DisengageLockon (Variables|Ref|GetAs%20BP%20Third%20Person%20Character))
              (Rendering|SetVisibility (Variables|Default|GetWBHealthBar) false false)
              (Collision|SetCollisionEnabled (Variables|Collision|GetCapsuleComponent) "NoCollision"))))))
    (else
      (Rendering|SetVisibility (Variables|Default|GetWBHealthBar) true false)
      (Components|Movement|StopMovementImmediately (Variables|Character|GetCharacterMovement))
      (bind _returnvalue (Animation|PlayAnimMontage "/Game/CourseWork/Enemy/Animations/Skele_Hit_Montage.Skele_Hit_Montage" 1.0 "None"))
      (Utilities|FlowControl|RetriggerableDelay _returnvalue)
      (Variables|State|SetBehavior "NewEnumerator3")
      (AI|Components|Blackboard|SetValueasEnum (AI|GetBlackboard 0) (Utilities|Name|MakeLiteralName "EBehavior") (Variables|State|GetBehavior)))))

(event EventOnDeselected
  ;[1 1 1] Lock On
  (Rendering|SetVisibility (Variables|Default|GetLockOn) false false))

(event EventOnSelected
  ;[1 1 1] Lock On
  (Rendering|SetVisibility (Variables|Default|GetLockOn) true false))

(fn ConstructionScript
  (bind _capsulecomponent (Variables|Collision|GetCapsuleComponent))
  (bind _relativelocation (Variables|/Script/Engine.SceneComponent|GetRelativeLocation _capsulecomponent))
  (bind (_x _y _z) (Math|Vector|BreakVector _relativelocation))
  (Transformation|SetWorldLocation (Variables|Character|GetMesh) (Math|Vector|MakeVector _x _y (- _z (Variables|/Script/Engine.CapsuleComponent|GetCapsuleHalfHeight _capsulecomponent))) false false))

(fn IsDead
  (return (Variables|Death|GetEnemyDead?)))